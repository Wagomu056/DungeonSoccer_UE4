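; Charge component that tracks a depletable resource with an overheat lockout and refill cycle, exposing its state and charge ratio.
; AffectChargeValue drains the charge, and an externally driven Update event runs a three-state machine: Can Action, Overheat, Recharging.
; Charge refills only after full depletion and a timed overheat delay, climbing at a constant rate until full restores Can Action.
; Debug prints mark each state transition.
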(event `self.ReceiveBeginPlay`
  (set `self.ChargeValue` (`self.ChargeMax`)))

(event `Event Update`
  (params (deltaTime :type "Float (double-precision)"))
  (switch `/Game/Blueprints/RechargeState` (`self.State`)
    (:`NewEnumerator0`
      (`self._UpdateCanAction`))
    (:`NewEnumerator1`
      (`self._UpdateOverheat` deltaTime))
    (:`NewEnumerator2`
      (`self._UpdateRecharging` deltaTime))))

(fn `_GetRechargeSpeed`
  (returns (RechargeSpeed :type "Float (double-precision)"))
  (return (/ (`self.ChargeMax`) (`self.RechargeTime`))))

(fn `_UpdateCanAction`
  (if (<= (`self.ChargeValue`) 0.0)
    (set `self.State` "NewEnumerator1")
    (`KismetSystemLibrary.PrintString` "ToOverHeat")))

(fn `_UpdateOverheat`
  (params (DeltaTime :type "Float (double-precision)"))
  (bind _output_get (set `self.OverheatTimer` (+ (`self.OverheatTimer`) DeltaTime)))
  (if (>= _output_get (`self.OverheatTime`))
    (set `self.OverheatTimer` 0.0)
    (set `self.State` "NewEnumerator2")
    (`KismetSystemLibrary.PrintString` "ToRecharging")))

(fn `_UpdateRecharging`
  (params (DeltaTime :type "Float (double-precision)"))
  (bind _output_get (set `self.ChargeValue` (+ (`self.ChargeValue`) (* (`self._GetRechargeSpeed`) DeltaTime))))
  (if (>= _output_get (`self.ChargeMax`))
    (set `self.ChargeValue` (`self.ChargeMax`))
    (set `self.State` "NewEnumerator0")
    (`KismetSystemLibrary.PrintString` "ToCanAction")))

(fn `AffectChargeValue`
  (params (SubValue :type "Float (double-precision)"))
  (bind _output_get (set `self.ChargeValue` (- (`self.ChargeValue`) SubValue)))
  (if (< _output_get 0.0)
    (set `self.ChargeValue` 0.0)))

(fn `GetChargePercent`
  (returns (ChargePercent :type "Float (double-precision)"))
  (return (/ (`self.ChargeValue`) (`self.ChargeMax`))))

(fn `GetState`
  (returns (State :type "/Game/Blueprints/RechargeState Enum"))
  (return (`self.State`)))