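; Weapon Blueprint for an automatic projectile gun with a recharge-based charge limit.
; PullTrigger fires once and starts a looping timer at RoundsPerSeconds, guarded by a DoN that ReleaseTrigger resets as it clears the timer.
; Fire checks CanShoot, whose recharge-state comparison appears unconnected, then plays sound, spawns a projectile and adjusts the charge.
; Tick updates RechargeComponent, and getters expose its state and charge percent.
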(event `PullTrigger`
  (`/Engine/EditorBlueprintResources/StandardMacros.Do N` 1 :!label _label
    (:`Exit`
      (`self.Fire`)
      (`KismetSystemLibrary.K2_SetTimer` null "Fire" (/ 1.0 (`self.RoundsPerSeconds`)) true))))

(event `ReleaseTrigger`
  (`KismetSystemLibrary.K2_ClearTimer` null "Fire")
  (goto _label :!via `Reset`))

(event `self.ReceiveTick`
  (params (DeltaSeconds :type "Float (single-precision)"))
  (`/Game/Blueprints/RechargeComponent.Event Update` (`self.RechargeComponent`) DeltaSeconds))

(event `Fire`
  (if (`|EnumEquality` (`/Game/Blueprints/RechargeComponent.GetState` (`self.RechargeComponent`)) "NewEnumerator0")
    (`GameplayStatics.SpawnSoundAttached` "/Game/Audio/weapon_shot.weapon_shot" (`self.GunMesh`) "None" (0.0 0.0 0.0) (struct) "KeepRelativeOffset" false 1.0 1.0 0.0 null null)
    (`|SpawnActorFromClass` "/Game/Blueprints/Projectile.Projectile_C" (`SceneComponent.K2_GetComponentToWorld` (`self.ProjectileSpawnPoint`)) "Undefined" "OverrideRootScale" null null)
    (`/Game/Blueprints/RechargeComponent.AffectChargeValue` (`self.RechargeComponent`) 1.0)))

(fn `GetChargePercent`
  (returns (ChargePercent :type "Float (double-precision)"))
  (return (`/Game/Blueprints/RechargeComponent.GetChargePercent` (`self.RechargeComponent`))))

(fn `GetRechargeState`
  (returns (State :type "/Game/Blueprints/RechargeState Enum"))
  (return (`/Game/Blueprints/RechargeComponent.GetState` (`self.RechargeComponent`))))

(fn `UserConstructionScript`)