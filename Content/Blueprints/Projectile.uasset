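; Projectile actor that damages what it hits, such as a laser shot.
; On overlap with an actor implementing IDamageable, it sends its Damage through an interface message unless that actor is tagged "friendly".
; Either way, it then plays a hit sound and laser spark emitter and destroys itself, while non-damageable actors are ignored.
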(event `self.ReceiveActorBeginOverlap`
  (params (OtherActor :type "Actor Object Reference"))
  (bind (_returnvalue_location _returnvalue_rotation) (`KismetMathLibrary.BreakTransform` (`self.GetTransform`)))
  (if (`KismetSystemLibrary.DoesImplementInterface` OtherActor "/Game/Blueprints/iDamageable.iDamageable_C")
    (if (not (`self.ActorHasTag` OtherActor "friendly"))
      (message `/Game/Blueprints/iDamageable.AffectHealth` OtherActor (`self.Damage`)))
    (`GameplayStatics.SpawnSoundAttached` "/Game/Audio/weapon_hit.weapon_hit" (`self.ProjectileCollision`) "None" (0.0 0.0 0.0) (struct) "KeepRelativeOffset" false 1.0 1.0 0.0 null null)
    (`GameplayStatics.SpawnEmitterAtLocation` "/Game/StarterContent/Particles/LaserSparks.LaserSparks" _returnvalue_location _returnvalue_rotation)
    (`self.K2_DestroyActor`)))

(fn `UserConstructionScript`)